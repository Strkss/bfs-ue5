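; BP_Spawner spawns a grid of BP_Cube actors when play begins.
; Nested loops over MaxRow and MaxCol place one cube per cell at a fixed 100-unit spacing, with columns along X and rows along Y.
; The offsets center the grid on the world origin at zero height, independent of the spawner's own transform, and each cube spawns regardless of collision.
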(event EventBeginPlay
  (for _index (range 0 (- (Variables|Default|GetMaxRow) 1))
    (for _index_2 (range 0 (- (Variables|Default|GetMaxCol) 1))
      (Game|SpawnActorfromClass "/Game/_BP/BP_Cube.BP_Cube_C" (Math|Transform|MakeTransform (Math|Vector|MakeVector (Math|Conversions|ToFloat(Integer) (+ (- (* _index_2 100) (* (Variables|Default|GetMaxCol) 50)) 50)) (Math|Conversions|ToFloat(Integer) (+ (- (* _index 100) (* (Variables|Default|GetMaxRow) 50)) 50)) 0.0)) "AlwaysSpawn" "MultiplyWithRoot" 0 0))))

(fn ConstructionScript)